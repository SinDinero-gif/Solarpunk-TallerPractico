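; Game mode for the Gardener game that handles level flow, UI setup and garage activation.
; On level start it creates the main menu or credits widget by level name, otherwise the energy bar via the game state, then after a short delay triggers actor spawning.
; Level completion opens the next level unless it is already current, and the game state's completed-work event activates the garage.
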(event `self.ReceiveBeginPlay`
  (bind _asgs_gardener_game_state (cast `/Game/Gardener/Core/GS_GardenerGameState` (`GameplayStatics.GetGameState`)))
  (set `self.GE_Gardener` _asgs_gardener_game_state)
  (add `self.OnLevelStarted` (delegate `OnLevelStarted_Event`))
  (add `self.OnLevelCompleted` (delegate `OnLevelCompleted_Event`))
  (add `/Game/Gardener/Core/GS_GardenerGameState.CompletedWork` (`self.GE_Gardener`) (delegate `Activate`)))

(event `Activate`
  (set `/Game/Gardener/Blueprints/WorkZones/BP_Garage.isActive` true (`/Game/Gardener/Core/GS_GardenerGameState.Garage Ref` (`self.GE_Gardener`)))
  (`KismetSystemLibrary.PrintString` "Garage Active" true true (struct :`R` 0.196938 :`G` 1.0 :`B` 0.044161 :`A` 1.0) 5.0))

(event `OnLevelStarted_Event`
  (bind _returnvalue (`GameplayStatics.GetCurrentLevelName` true))
  (`self.LoadUI` _returnvalue)
  (`KismetSystemLibrary.Delay` 1.0)
  (`/Game/Gardener/Core/GS_GardenerGameState.SpawnActorsInLevel_Event` (`self.GE_Gardener`)))

(event `OnLevelCompleted_Event` :!signature `self.OnLevelCompleted`
  (params (nextLevelName :type String))
  (`self.LoadLevel` nextLevelName))

(fn `LoadLevel`
  (params (levelName :type String))
  (bind _returnvalue (`GameplayStatics.GetCurrentLevelName` true))
  (if (not (== _returnvalue levelName))
    (`GameplayStatics.OpenLevel` (`KismetStringLibrary.Conv_StringToName` levelName))))

(fn `LoadUI`
  (params (currentLevelName :type String))
  (bind _returnvalue (`GameplayStatics.GetPlayerController` 0))
  (if (== currentLevelName "MainMenu")
    (bind _returnvalue_2 (`|CreateWidget` "/Game/Gardener/Blueprints/UIAssets/MainMenu.MainMenu_C" _returnvalue))
    (`UserWidget.AddToViewport` _returnvalue_2 0)
    (elif (== currentLevelName "Credits")
      (bind _returnvalue_3 (`|CreateWidget` "/Game/Gardener/Blueprints/UIAssets/CreditsMenu.CreditsMenu_C" _returnvalue))
      (`UserWidget.AddToViewport` _returnvalue_3 0)
      (else
        (`/Game/Gardener/Core/GS_GardenerGameState.CreateEnergyBarEvent` (`self.GE_Gardener`))))))

(fn `UserConstructionScript`
  (`parent.UserConstructionScript`))