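; Cuco is a two-player shared vehicle whose players take Movement, Task or Energy stations to drive, collect and spray water, or spawn energy pods.
; Station-checked inputs push and turn a physics sphere, with a lagging spring arm and Niagara effects.
; Paused and resumed looping timers drain energy and send water to a work base.
; Empty energy stops thrust, fades to black and reloads the level.
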(event `StopCarEvent`
  (`self.inputStop`)
  (`|ExecutionSequence`
    (:`then_0`
      (`PlayerCameraManager.StartCameraFade` (`GameplayStatics.GetPlayerCameraManager` 0) 0.0 2.0 4.0 (struct :`A` 1.0) false false))
    (:`then_1`
      (`KismetSystemLibrary.Delay` 3.8)
      (bind _returnvalue (`GameplayStatics.GetCurrentLevelName` true))
      (`GameplayStatics.OpenLevel` (`KismetStringLibrary.Conv_StringToName` _returnvalue)))))

(event `self.ReceiveBeginPlay`
  (`|ExecutionSequence`
    (:`then_0`
      (`KismetArrayLibrary.Array_Add` (`self.WaterStreamsArray`) (`self.WaterStream1`))
      (`KismetArrayLibrary.Array_Add` (`self.WaterStreamsArray`) (`self.WaterStream2`))
      (`KismetArrayLibrary.Array_Add` (`self.WaterStreamsArray`) (`self.WaterStream3`))
      (`KismetArrayLibrary.Array_Add` (`self.WaterStreamsArray`) (`self.WaterStream4`))
      (`KismetArrayLibrary.Array_Add` (`self.WaterStreamsArray`) (`self.WaterStream5`))
      (`KismetArrayLibrary.Array_Add` (`self.WaterStreamsArray`) (`self.WaterStream6`)))
    (:`then_1`
      (bind _asgs_gardener_game_state (cast `/Game/Gardener/Core/GS_GardenerGameState` (`GameplayStatics.GetGameState`)))
      (set `self.GS Gardener Game State` _asgs_gardener_game_state))
    (:`then_2`
      (`KismetSystemLibrary.PrintString` (`KismetStringLibrary.Concat_StrStr` "Has Water:" (`KismetStringLibrary.Conv_BoolToString` (`self.hasWater`))))
      (`PlayerCameraManager.StartCameraFade` (`GameplayStatics.GetPlayerCameraManager` 0) 4.0 0.0 4.0 (struct :`A` 1.0) false false))
    (:`then_3`
      (bind _returnvalue (`KismetSystemLibrary.K2_SetTimerDelegate` (delegate `useEnergyEvent`) 0.2 true))
      (set `self.EnergyEventHandle` _returnvalue))
    (:`then_4`
      (bind _returnvalue_2 (`KismetSystemLibrary.K2_SetTimerDelegate` (delegate `Usar Agua del Carro`) 0.2 true))
      (bind _output_get (set `self.sendWaterHandle` _returnvalue_2))
      (`KismetSystemLibrary.K2_PauseTimerHandle` _output_get))
    (:`then_5`
      (`NiagaraComponent.SetPaused` (`self.NS_CarRings`) true))
    (:`then_6`
      (for _array_element (`self.WaterStreamsArray`)
        (`NiagaraComponent.SetPaused` _array_element true)))))

(event `useEnergyEvent`
  (`self.useCurrentEnergy` (`self.Subtracted Energy`)))

(event `/Game/Gardener/Blueprints/Interfaces/I_charging.sendCharge`
  (params (amount :type "Float (double-precision)"))
  (`self.addCurrentEnergy` amount))

(event `Usar Agua del Carro`
  (bind _subtracted_water (`self.Subtracted Water`))
  (`self.Use Current Water` _subtracted_water)
  (`/Game/Gardener/Blueprints/Interfaces/I_charging.sendWater` (`self.WorkBaseRef`) _subtracted_water (`self.isUsingWater`) "NewEnumerator0"))

(event `/Game/Gardener/Blueprints/Interfaces/I_charging.sendResource`
  (params (amount :type "Float (double-precision)") (resourceType :type "/Game/Gardener/Blueprints/Interfaces/Enums/EResources Enum" :default "NewEnumerator0"))
  (if (`self.isGettingResource`)
    (switch `/Game/Gardener/Blueprints/Interfaces/Enums/EResources` resourceType
      (:`NewEnumerator0`
        (`self.Add Water` amount)))))

(event `self.ReceiveTick`
  (params (DeltaSeconds :type "Float (single-precision)"))
  (bind _springarm (`self.SpringArm`))
  (`|ExecutionSequence`
    (:`then_0`
      (if (<= (`self.currentEnergy`) 0.0)
        (`self.StopCarEvent`)))
    (:`then_1`
      (if (> (`self.currentWater`) 0.0)
        (set `self.hasWater` true)
        (else
          (set `self.hasWater` false))))
    (:`then_2`
      (`SceneComponent.K2_SetWorldLocation` _springarm (`KismetMathLibrary.VInterpTo` (`SceneComponent.K2_GetComponentLocation` _springarm) (`self.K2_GetActorLocation`) (`GameplayStatics.GetWorldDeltaSeconds`) 4.0) false false))))

(event `EnhancedInput|/Game/Gardener/Blueprints/Vehicles/InputsPlayer/Actions/IA_Player2Movement`
  (params (ActionValue :type "Float (double-precision)") (ElapsedSeconds :type "Float (double-precision)") (TriggeredSeconds :type "Float (double-precision)") (InputAction :type "InputAction Object Reference" :default "/Game/Gardener/Blueprints/Vehicles/InputsPlayer/Actions/IA_Player2Movement.IA_Player2Movement"))
  (bind _energyeventhandle (`self.EnergyEventHandle`))
  (bind _ns_carrings (`self.NS_CarRings`))
  ;[1 1 1] Player 2 Movement System
  (:`Triggered`
    (bind _outvalue (`self.Check Station` (`self.player2 Station`) 2 "Movement"))
    (if _outvalue
      (`PrimitiveComponent.AddForce` (`self.Sphere`) (* (`SceneComponent.GetForwardVector` (`self.Sphere`)) ActionValue (`self.CarSpeed`)) "None" true)
      (`KismetSystemLibrary.K2_UnPauseTimerHandle` _energyeventhandle)
      (if (> ActionValue 0.0)
        (`ActorComponent.Activate` _ns_carrings false)
        (`NiagaraComponent.SetPaused` _ns_carrings false)
        (else
          (`ActorComponent.Deactivate` _ns_carrings :!label _label)))
      (else
        (`KismetSystemLibrary.PrintString` "Wrong Station" true true (struct :`R` 1.0 :`B` 0.023615 :`A` 1.0) 5.0)
        (`KismetSystemLibrary.K2_PauseTimerHandle` _energyeventhandle))))
  (:`Completed`
    (goto _label)))

(event `EnhancedInput|/Game/Gardener/Blueprints/Vehicles/InputsPlayer/Actions/IA_Player1Movement`
  (params (ActionValue :type "Float (double-precision)") (ElapsedSeconds :type "Float (double-precision)") (TriggeredSeconds :type "Float (double-precision)") (InputAction :type "InputAction Object Reference" :default "/Game/Gardener/Blueprints/Vehicles/InputsPlayer/Actions/IA_Player1Movement.IA_Player1Movement"))
  (bind _energyeventhandle (`self.EnergyEventHandle`))
  (bind _ns_carrings (`self.NS_CarRings`))
  (bind _engine (`self.Engine`))
  ;[1 1 1] Player 1 Movement System
  (:`Triggered`
    (bind _outvalue (`self.Check Station` (`self.player1 Station`) 1 "Movement"))
    (if _outvalue
      (`PrimitiveComponent.AddForce` (`self.Sphere`) (* (`SceneComponent.GetForwardVector` (`self.Sphere`)) ActionValue (`self.CarSpeed`)) "None" true)
      (`KismetSystemLibrary.K2_UnPauseTimerHandle` _energyeventhandle)
      (if (> ActionValue 0.0)
        (`ActorComponent.Activate` _ns_carrings false)
        (`NiagaraComponent.SetPaused` _ns_carrings false)
        (`AudioParameterControllerInterface.SetTriggerParameter` _engine "in")
        (else
          (`ActorComponent.Deactivate` _ns_carrings :!label _label_2)
          (`AudioParameterControllerInterface.SetTriggerParameter` _engine "out")))
      (else
        (`KismetSystemLibrary.PrintString` "Wrong Station" true true (struct :`R` 1.0 :`B` 0.023615 :`A` 1.0) 5.0)
        (`KismetSystemLibrary.K2_PauseTimerHandle` _energyeventhandle))))
  (:`Completed`
    (goto _label_2)))

(event `EnhancedInput|/Game/Gardener/Blueprints/Vehicles/InputsPlayer/Actions/IA_Sides`
  (params (ActionValue :type "Float (double-precision)") (ElapsedSeconds :type "Float (double-precision)") (TriggeredSeconds :type "Float (double-precision)") (InputAction :type "InputAction Object Reference" :default "/Game/Gardener/Blueprints/Vehicles/InputsPlayer/Actions/IA_Sides.IA_Sides"))
  ;[1 1 1] Player 1 Movement System
  (:`Triggered`
    (bind _outvalue (`self.Check Station` (`self.player1 Station`) 1 "Movement" :!label _label_3))
    (if _outvalue
      (`PrimitiveComponent.SetPhysicsAngularVelocityInDegrees` (`self.Sphere`) (`KismetMathLibrary.MakeVector` 0.0 0.0 (* ActionValue (`self.carRotationSpeed`))) true "None")))
  (:`Completed`
    (goto _label_3)))

(event `EnhancedInput|/Game/Gardener/Blueprints/Vehicles/InputsPlayer/Actions/IA_Float`
  (params (ActionValue :type "Float (double-precision)") (ElapsedSeconds :type "Float (double-precision)") (TriggeredSeconds :type "Float (double-precision)") (InputAction :type "InputAction Object Reference" :default "/Game/Gardener/Blueprints/Vehicles/InputsPlayer/Actions/IA_Float.IA_Float"))
  ;[1 1 1] Player 1 Movement System
  (:`Triggered`
    (bind _outvalue (`self.Check Station` (`self.player1 Station`) 1 "Movement" :!label _label_4))
    (if _outvalue
      (`PrimitiveComponent.AddForce` (`self.Sphere`) (* (`SceneComponent.GetUpVector` (`self.Sphere`)) ActionValue (`self.carFloatSpeed`)) "None" true)
      (else
        (`KismetSystemLibrary.PrintString` "Wrong Station" true true (struct :`R` 1.0 :`B` 0.023615 :`A` 1.0) 5.0))))
  (:`Completed`
    (goto _label_4)))

(event `EnhancedInput|/Game/Gardener/Blueprints/Vehicles/InputsPlayer/Actions/IA_Float2`
  (params (ActionValue :type "Float (double-precision)") (ElapsedSeconds :type "Float (double-precision)") (TriggeredSeconds :type "Float (double-precision)") (InputAction :type "InputAction Object Reference" :default "/Game/Gardener/Blueprints/Vehicles/InputsPlayer/Actions/IA_Float2.IA_Float2"))
  ;[1 1 1] Player 2 Movement System
  (:`Triggered`
    (bind _outvalue (`self.Check Station` (`self.player2 Station`) 2 "Movement" :!label _label_5))
    (if _outvalue
      (`PrimitiveComponent.AddForce` (`self.Sphere`) (* (`SceneComponent.GetUpVector` (`self.Sphere`)) ActionValue (`self.carFloatSpeed`)) "None" true)
      (else
        (`KismetSystemLibrary.PrintString` "Wrong Station" true true (struct :`R` 1.0 :`B` 0.023615 :`A` 1.0) 5.0))))
  (:`Completed`
    (goto _label_5)))

(event `EnhancedInput|/Game/Gardener/Blueprints/Vehicles/InputsPlayer/Actions/IA_Sides2`
  (params (ActionValue :type "Float (double-precision)") (ElapsedSeconds :type "Float (double-precision)") (TriggeredSeconds :type "Float (double-precision)") (InputAction :type "InputAction Object Reference" :default "/Game/Gardener/Blueprints/Vehicles/InputsPlayer/Actions/IA_Sides2.IA_Sides2"))
  ;[1 1 1] Player 2 Movement System
  (:`Triggered`
    (bind _outvalue (`self.Check Station` (`self.player2 Station`) 2 "Movement" :!label _label_6))
    (if _outvalue
      (`PrimitiveComponent.SetPhysicsAngularVelocityInDegrees` (`self.Sphere`) (`KismetMathLibrary.MakeVector` 0.0 0.0 (* ActionValue (`self.carRotationSpeed`))) true "None")))
  (:`Completed`
    (goto _label_6)))

(event `EnhancedInput|/Game/Gardener/Blueprints/Vehicles/InputsPlayer/Actions/IA_PlayerState2`
  (params (ActionValue :type Boolean) (ElapsedSeconds :type "Float (double-precision)") (TriggeredSeconds :type "Float (double-precision)") (InputAction :type "InputAction Object Reference" :default "/Game/Gardener/Blueprints/Vehicles/InputsPlayer/Actions/IA_PlayerState2.IA_PlayerState2"))
  ;[1 1 1] Player 2 Assignation
  (:`Started`
    (bind (_inputset _playerstation) (`/Game/VehicleTemplate/Blueprints/VehiclePlayerController.assignPlayerToStation` (`/Game/Gardener/Blueprints/Vehicles/InputsPlayer/PS_VehiclePlayerState.As Vehicle Player Controller` (`/Game/Gardener/Core/GS_GardenerGameState.As PS Vehicle Player State` (`self.GS Gardener Game State`))) 2))
    (bind _output_get (set `self.player2 Station` _playerstation))
    (if (== (`.currentPlayer_14_F96142CE4E964300460AC7980138A589` (break `/Game/Gardener/Blueprints/Interfaces/s_Station` _output_get)) 2)
      (`KismetSystemLibrary.PrintString` (`KismetStringLibrary.Concat_StrStr` "2  " (break `/Game/Gardener/Blueprints/Interfaces/s_Station` _output_get)) true true (struct :`G` 0.017333 :`B` 1.0 :`A` 1.0) 5.0)
      (bind _stationoutput (`self.Set Station Enum` (break `/Game/Gardener/Blueprints/Interfaces/s_Station` _output_get)))
      (`/Game/Gardener/Blueprints/Resources/WBP_EnergyBar.Rotate Action2` (`/Game/Gardener/Core/GS_GardenerGameState.EnergyBarRef` (`self.GS Gardener Game State`)) _stationoutput)
      (else
        (`KismetSystemLibrary.PrintString` "Player 2 isn't Setted" true true (struct :`R` 1.0 :`G` 0.040508 :`B` 0.020612 :`A` 1.0) 5.0)))))

(event `EnhancedInput|/Game/Gardener/Blueprints/Vehicles/InputsPlayer/Actions/IA_PlayerState`
  (params (ActionValue :type Boolean) (ElapsedSeconds :type "Float (double-precision)") (TriggeredSeconds :type "Float (double-precision)") (InputAction :type "InputAction Object Reference" :default "/Game/Gardener/Blueprints/Vehicles/InputsPlayer/Actions/IA_PlayerState.IA_PlayerState"))
  ;[1 1 1] Player 1 Assignation
  (:`Started`
    (bind (_inputset _playerstation) (`/Game/VehicleTemplate/Blueprints/VehiclePlayerController.assignPlayerToStation` (`/Game/Gardener/Blueprints/Vehicles/InputsPlayer/PS_VehiclePlayerState.As Vehicle Player Controller` (`/Game/Gardener/Core/GS_GardenerGameState.As PS Vehicle Player State` (`self.GS Gardener Game State`))) 1))
    (bind _output_get (set `self.player1 Station` _playerstation))
    (if (== (`.currentPlayer_14_F96142CE4E964300460AC7980138A589` (break `/Game/Gardener/Blueprints/Interfaces/s_Station` _output_get)) 1)
      (`KismetSystemLibrary.PrintString` (`KismetStringLibrary.Concat_StrStr` "1 " (break `/Game/Gardener/Blueprints/Interfaces/s_Station` _output_get)) true true (struct :`G` 0.017333 :`B` 1.0 :`A` 1.0) 5.0)
      (bind _stationoutput (`self.Set Station Enum` (break `/Game/Gardener/Blueprints/Interfaces/s_Station` _output_get)))
      (`/Game/Gardener/Blueprints/Resources/WBP_EnergyBar.Rotate Action1` (`/Game/Gardener/Core/GS_GardenerGameState.EnergyBarRef` (`self.GS Gardener Game State`)) _stationoutput)
      (else
        (`KismetSystemLibrary.PrintString` "Player 2 isn't Setted" true true (struct :`R` 1.0 :`G` 0.040508 :`B` 0.020612 :`A` 1.0) 5.0)))))

(event `EnhancedInput|/Game/Gardener/Blueprints/Vehicles/InputsPlayer/Actions/IA_Pod`
  (params (ActionValue :type Boolean) (ElapsedSeconds :type "Float (double-precision)") (TriggeredSeconds :type "Float (double-precision)") (InputAction :type "InputAction Object Reference" :default "/Game/Gardener/Blueprints/Vehicles/InputsPlayer/Actions/IA_Pod.IA_Pod"))
  (bind _returnvalue (`SceneComponent.K2_GetComponentToWorld` (`self.CarMesh`)))
  ;[1 1 1] Player Energy Pod
  (:`Started`
    (bind _outvalue (`self.Check Station` (`self.player1 Station`) 1 "Energy"))
    (bind _outvalue_2 (`self.Check Station` (`self.player2 Station`) 2 "Energy"))
    (if (or _outvalue _outvalue_2)
      (bind _canspawn (`/Game/Gardener/Core/GS_GardenerGameState.spawnEnergyPod` (`self.GS Gardener Game State`) ActionValue))
      (if _canspawn
        (`|SpawnActorFromClass` "/Game/Gardener/Blueprints/Resources/Energy/BP_EnergyZone_Spawnable.BP_EnergyZone_Spawnable_C" (`KismetMathLibrary.MakeTransform` (`KismetMathLibrary.MakeVector` (.x (.location _returnvalue)) (.y (.location _returnvalue)) (+ (.z (.location _returnvalue)) 300.0))) "Undefined" "MultiplyWithRoot" null 400.0 5.0 null)))))

(event `EnhancedInput|/Game/Gardener/Blueprints/Vehicles/InputsPlayer/Actions/IA_ColletWater`
  (params (ActionValue :type "Float (double-precision)") (ElapsedSeconds :type "Float (double-precision)") (TriggeredSeconds :type "Float (double-precision)") (InputAction :type "InputAction Object Reference" :default "/Game/Gardener/Blueprints/Vehicles/InputsPlayer/Actions/IA_ColletWater.IA_ColletWater"))
  (bind _energyeventhandle (`self.EnergyEventHandle`))
  ;[1 1 1] Player 1 Task collet
  (:`Started`
    (bind _outvalue (`self.Check Station` (`self.player1 Station`) 1 "Task"))
    (if _outvalue
      (set `self.Subtracted Energy` 0.2)
      (set `self.isGettingResource` true)
      (`KismetSystemLibrary.K2_UnPauseTimerHandle` _energyeventhandle)
      (set `self.currentWater` (`KismetMathLibrary.FClamp` (`self.currentWater`) 0.0 100.0))))
  (:`Completed`
    (set `self.Subtracted Energy` 0.05)
    (set `self.isGettingResource` false)
    (`KismetSystemLibrary.K2_PauseTimerHandle` _energyeventhandle)))

(event `EnhancedInput|/Game/Gardener/Blueprints/Vehicles/InputsPlayer/Actions/IA_ColletWater2`
  (params (ActionValue :type "Float (double-precision)") (ElapsedSeconds :type "Float (double-precision)") (TriggeredSeconds :type "Float (double-precision)") (InputAction :type "InputAction Object Reference" :default "/Game/Gardener/Blueprints/Vehicles/InputsPlayer/Actions/IA_ColletWater2.IA_ColletWater2"))
  (bind _energyeventhandle (`self.EnergyEventHandle`))
  ;[1 1 1] Player 2 Task collet
  (:`Started`
    (bind _outvalue (`self.Check Station` (`self.player2 Station`) 2 "Task"))
    (if _outvalue
      (set `self.Subtracted Energy` 0.2)
      (set `self.isGettingResource` true)
      (`KismetSystemLibrary.K2_UnPauseTimerHandle` _energyeventhandle)
      (set `self.currentWater` (`KismetMathLibrary.FClamp` (`self.currentWater`) 0.0 100.0))))
  (:`Completed`
    (set `self.Subtracted Energy` 0.05)
    (set `self.isGettingResource` false)
    (`KismetSystemLibrary.K2_PauseTimerHandle` _energyeventhandle)))

(event `EnhancedInput|/Game/Gardener/Blueprints/Vehicles/InputsPlayer/Actions/IA_ColletWater`
  (params (ActionValue :type "Float (double-precision)") (ElapsedSeconds :type "Float (double-precision)") (TriggeredSeconds :type "Float (double-precision)") (InputAction :type "InputAction Object Reference" :default "/Game/Gardener/Blueprints/Vehicles/InputsPlayer/Actions/IA_ColletWater.IA_ColletWater"))
  (bind _energyeventhandle (`self.EnergyEventHandle`))
  ;[1 1 1] Player 1 Task collet
  (:`Started`
    (bind _outvalue (`self.Check Station` (`self.player1 Station`) 1 "Task"))
    (if _outvalue
      (set `self.Subtracted Energy` 0.2)
      (set `self.isGettingResource` true)
      (`KismetSystemLibrary.K2_UnPauseTimerHandle` _energyeventhandle)
      (set `self.currentWater` (`KismetMathLibrary.FClamp` (`self.currentWater`) 0.0 100.0))))
  (:`Completed`
    (set `self.Subtracted Energy` 0.05)
    (set `self.isGettingResource` false)
    (`KismetSystemLibrary.K2_PauseTimerHandle` _energyeventhandle)))

(event `EnhancedInput|/Game/Gardener/Blueprints/Vehicles/InputsPlayer/Actions/IA_ThrowWater`
  (params (ActionValue :type "Float (double-precision)") (ElapsedSeconds :type "Float (double-precision)") (TriggeredSeconds :type "Float (double-precision)") (InputAction :type "InputAction Object Reference" :default "/Game/Gardener/Blueprints/Vehicles/InputsPlayer/Actions/IA_ThrowWater.IA_ThrowWater"))
  (bind _energyeventhandle (`self.EnergyEventHandle`))
  (bind _sendwaterhandle (`self.sendWaterHandle`))
  (bind _waterstreamsarray (`self.WaterStreamsArray`))
  ;[0.1714 0.3005 0.8148] Player 1 task Trhow
  (:`Started`
    (bind _outvalue (`self.Check Station` (`self.player1 Station`) 1 "Task"))
    (if _outvalue
      (set `self.Subtracted Energy` 0.2)
      (if (`self.hasWater`)
        (set `self.isUsingWater` true)
        (`KismetSystemLibrary.K2_UnPauseTimerHandle` _energyeventhandle)
        (`KismetSystemLibrary.PrintString` "Using Resource" true true (struct :`G` 1.0 :`B` 0.09332 :`A` 1.0) 4.0)
        (`KismetSystemLibrary.K2_UnPauseTimerHandle` _sendwaterhandle)
        (for _array_element _waterstreamsarray
          (`ActorComponent.Activate` _array_element false)
          (`NiagaraComponent.SetPaused` _array_element false))
        (else
          (set `self.isUsingWater` false)
          (`KismetSystemLibrary.PrintString` "There isn't a Resource")
          (`KismetSystemLibrary.K2_PauseTimerHandle` _energyeventhandle)
          (`KismetSystemLibrary.K2_PauseTimerHandle` _sendwaterhandle)
          (for _array_element_2 _waterstreamsarray :!label _label_7
            (`ActorComponent.Deactivate` _array_element_2))))))
  (:`Completed`
    (set `self.Subtracted Energy` 0.05)
    (set `self.isUsingWater` false)
    (`KismetSystemLibrary.K2_PauseTimerHandle` _energyeventhandle)
    (`KismetSystemLibrary.K2_PauseTimerHandle` _sendwaterhandle)
    (goto _label_7)))

(event `EnhancedInput|/Game/Gardener/Blueprints/Vehicles/InputsPlayer/Actions/IA_ThrowWater2`
  (params (ActionValue :type Boolean) (ElapsedSeconds :type "Float (double-precision)") (TriggeredSeconds :type "Float (double-precision)") (InputAction :type "InputAction Object Reference" :default "/Game/Gardener/Blueprints/Vehicles/InputsPlayer/Actions/IA_ThrowWater2.IA_ThrowWater2"))
  (bind _energyeventhandle (`self.EnergyEventHandle`))
  (bind _waterstreamsarray (`self.WaterStreamsArray`))
  (bind _sendwaterhandle (`self.sendWaterHandle`))
  ;[0.1714 0.3005 0.8148] Player 1 task Trhow
  (:`Started`
    (bind _outvalue (`self.Check Station` (`self.player2 Station`) 2 "Task"))
    (if _outvalue
      (set `self.Subtracted Energy` 0.2)
      (if (`self.hasWater`)
        (set `self.isUsingWater` true)
        (`KismetSystemLibrary.K2_UnPauseTimerHandle` _energyeventhandle)
        (`KismetSystemLibrary.PrintString` "Using Resource" true true (struct :`G` 1.0 :`B` 0.09332 :`A` 1.0) 4.0)
        (`KismetSystemLibrary.K2_UnPauseTimerHandle` _sendwaterhandle)
        (for _array_element _waterstreamsarray
          (`ActorComponent.Activate` _array_element false)
          (`NiagaraComponent.SetPaused` _array_element false))
        (else
          (set `self.isUsingWater` false)
          (`KismetSystemLibrary.PrintString` "There isn't a Resource")
          (`KismetSystemLibrary.K2_PauseTimerHandle` _energyeventhandle)
          (`KismetSystemLibrary.K2_PauseTimerHandle` _sendwaterhandle)
          (for _array_element_2 _waterstreamsarray :!label _label_8
            (`ActorComponent.Deactivate` _array_element_2))))))
  (:`Completed`
    (set `self.Subtracted Energy` 0.05)
    (set `self.isUsingWater` false)
    (`KismetSystemLibrary.K2_PauseTimerHandle` _energyeventhandle)
    (`KismetSystemLibrary.K2_PauseTimerHandle` _sendwaterhandle)
    (goto _label_8)))

(fn `Add Water`
  (params (amount :type "Float (double-precision)"))
  (set `self.currentWater` (`KismetMathLibrary.FClamp` (+ (`self.currentWater`) amount) 0.0 100.0)))

(fn `addCurrentEnergy`
  (params (energyToAdd :type "Float (double-precision)"))
  (set `self.currentEnergy` (`KismetMathLibrary.FClamp` (+ (`self.currentEnergy`) energyToAdd) 0.0 100.0)))

(fn `carEngineShift`
  (params (`pitch change` :type "Float (double-precision)"))
  (`AudioParameterControllerInterface.SetFloatParameter` (`self.Engine`) "EngineTone" `pitch change`))

(fn `Check Station`
  (params (`Player Station` :type "/Game/Gardener/Blueprints/Interfaces/s_Station Structure") (playerIndex :type Integer) (`station Name` :type String))
  (returns (outValue :type Boolean))
  (bind (_name _currentplayer) (break `/Game/Gardener/Blueprints/Interfaces/s_Station` `Player Station`))
  (if (== _currentplayer playerIndex)
    (return (`KismetStringLibrary.EqualEqual_StrStr` _name `station Name`))
    (else
      (`KismetSystemLibrary.PrintString` "Different Player Index"))))

(fn `inputStop`
  (`|ExecutionSequence`
    (:`then_0`
      (set `self.CarSpeed` 0.0))
    (:`then_1`
      (return))))

(fn `Set Station Enum`
  (params (StationName :type String))
  (returns (StationOutput :type "/Game/Gardener/Blueprints/Vehicles/InputsPlayer/EnumState/ENUM_StatePositions Enum"))
  (switch `string` StationName
    (:`Movement`
      (set `self.LastPlayerStation` "NewEnumerator0"))
    (:`Task`
      (set `self.LastPlayerStation` "NewEnumerator2"))
    (:`Energy`
      (set `self.LastPlayerStation` "NewEnumerator1")))
  (return (`self.LastPlayerStation`)))

(fn `Use Current Water`
  (params (amount :type "Float (double-precision)"))
  (set `self.currentWater` (`KismetMathLibrary.FClamp` (- (`self.currentWater`) amount) 0.0 100.0)))

(fn `useCurrentEnergy`
  (params (subtractedEnergy :type "Float (double-precision)"))
  (set `self.currentEnergy` (- (`self.currentEnergy`) subtractedEnergy)))

(fn `UserConstructionScript`)