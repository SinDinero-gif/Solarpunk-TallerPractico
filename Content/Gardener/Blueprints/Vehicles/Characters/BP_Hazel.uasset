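; BP_Hazel is the Hazel character, who celebrates when a work zone is completed.
; On BeginPlay it attaches a face plane to the mesh's face socket, creates a dynamic material for it and binds to the game state's completed work zone event.
; Celebrate swaps the face texture and plays a montage, then on completion changes the face again and unbinds, so later completions are ignored.
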(event `self.ReceiveBeginPlay`
  (bind _faceplane (`self.FacePlane`))
  (`SceneComponent.K2_AttachToComponent` _faceplane (`self.Hazel Mesh`) "Face_Socket" "KeepRelative" "KeepRelative" "KeepRelative" true)
  (bind _returnvalue (`PrimitiveComponent.CreateDynamicMaterialInstance` (`self.FacePlane`) 0 (`PrimitiveComponent.GetMaterial` _faceplane 0) "None"))
  (set `self.DynamicFaceTxt` _returnvalue)
  (bind _asgs_gardener_game_state (cast `/Game/Gardener/Core/GS_GardenerGameState` (`GameplayStatics.GetGameState`)))
  (bind _output_get (set `self.GameState` _asgs_gardener_game_state))
  (add `/Game/Gardener/Core/GS_GardenerGameState.CompletedWorkZone` _output_get (delegate `Celebrate`)))

(event `Celebrate`
  (`MaterialInstanceDynamic.SetTextureParameterValue` (`self.DynamicFaceTxt`) "face_Text" "/Game/Gardener/Textures/Hazel/Expresions_Hazel/Hazel__13_.Hazel__13_")
  (`|PlayMontage` (`self.Hazel Mesh`) "/Game/Gardener/Animations/Hazel/Hazel_celebracion_01_escala_animation_Montage.Hazel_celebracion_01_escala_animation_Montage"
    (:`OnCompleted`
      (`MaterialInstanceDynamic.SetTextureParameterValue` (`self.DynamicFaceTxt`) "face_Text" "/Game/Gardener/Textures/Hazel/Expresions_Hazel/Hazel__8_.Hazel__8_")
      (remove `/Game/Gardener/Core/GS_GardenerGameState.CompletedWorkZone` (`self.GameState`) (delegate `Celebrate`)))))

(fn `UserConstructionScript`)