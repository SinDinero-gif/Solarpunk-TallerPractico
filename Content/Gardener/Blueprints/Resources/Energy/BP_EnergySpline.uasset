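; Spline-based energy road that sends charge messages to an overlapping actor.
; The construction script builds spline meshes between the Road's points and spaces box colliders along its length by segment count, keeping the last in BoxCollider.
; A looping timer started at BeginPlay sends EnergyAmount to the overlap event's OtherActor.
; BoxCollider's begin and end overlap events unpause and pause that timer.
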(event `self.ReceiveBeginPlay`
  (bind _returnvalue (`KismetSystemLibrary.K2_SetTimerDelegate` (delegate `LoadEnergyEvent`) 0.5 true))
  (set `self.TimerHandler` _returnvalue))

(event `LoadEnergyEvent`
  (message `/Game/Gardener/Blueprints/Interfaces/I_charging.sendCharge` (stale `self.BoxCollider.OnComponentBeginOverlap` OtherActor) (`self.Energy Amount`)))

(event `self.BoxCollider.OnComponentBeginOverlap`
  (params (OverlappedComponent :type "PrimitiveComponent Object Reference") (OtherActor :type "Actor Object Reference") (OtherComp :type "PrimitiveComponent Object Reference") (OtherBodyIndex :type Integer) (bFromSweep :type Boolean) (SweepResult :type "HitResult Structure (by ref)"))
  (`KismetSystemLibrary.K2_UnPauseTimerHandle` (`self.TimerHandler`)))

(event `self.BoxCollider.OnComponentEndOverlap`
  (params (OverlappedComponent :type "PrimitiveComponent Object Reference") (OtherActor :type "Actor Object Reference") (OtherComp :type "PrimitiveComponent Object Reference") (OtherBodyIndex :type Integer))
  (`KismetSystemLibrary.K2_PauseTimerHandle` (`self.TimerHandler`)))

(fn `UserConstructionScript`
  (bind _road (`self.Road`))
  (for _index (range (+ (- (`SplineComponent.GetNumberOfSplinePoints` (`self.Road`)) 2) 1))
    ;[1 1 1] Mesh
    (bind _returnvalue (`AddComponent|NODE_AddSplineMeshComponent-0`))
    (bind (_location _tangent) (`SplineComponent.GetLocationAndTangentAtSplinePoint` _road _index "Local"))
    (bind (_location_2 _tangent_2) (`SplineComponent.GetLocationAndTangentAtSplinePoint` _road (+ _index 1) "Local"))
    (`SplineMeshComponent.SetStartAndEnd` _returnvalue _location _tangent _location_2 _tangent_2 true)
    (`SceneComponent.K2_AttachToComponent` _returnvalue (`self.DefaultSceneRoot`) "None" "KeepRelative" "KeepRelative" "KeepRelative" true))
  (for _index_2 (range (+ (`self.segments`) 1))
    (bind (_returnvalue_location _returnvalue_rotation) (`KismetMathLibrary.BreakTransform` (`SplineComponent.GetTransformAtDistanceAlongSpline` (`self.Road`) (* _index_2 (/ (`SplineComponent.GetSplineLength` (`self.Road`)) (`self.segments`))) "Local" false)))
    (bind _returnvalue_2 (`AddComponent|NODE_AddBoxComponent-2` :`RelativeTransform` (`KismetMathLibrary.MakeTransform` _returnvalue_location _returnvalue_rotation (`self.Relative Transform Scale`))))
    (set `self.BoxCollider` _returnvalue_2)))