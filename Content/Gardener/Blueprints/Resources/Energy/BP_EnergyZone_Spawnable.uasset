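; BP_EnergyZone_Spawnable is an energy zone resource actor, named as a spawnable variant, that animates its mesh vertically.
; On BeginPlay it runs the parent logic, unpauses the TimerHandler timer and plays a timeline from the start.
; Each timeline update adds the Seno track value to the static mesh's current relative Z with sweep, so offsets accumulate rather than offset a fixed origin.
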(event `self.ReceiveBeginPlay`
  (bind (_relativelocation_x _relativelocation_y _relativelocation_z) (`KismetMathLibrary.BreakVector` (`SceneComponent.RelativeLocation` (`self.StaticMesh`))))
  (`parent.ReceiveBeginPlay`)
  (`KismetSystemLibrary.K2_UnPauseTimerHandle` (`self.timerHandler`))
  (bind (_direction _seno) (`Timeline|Timeline` :!via `PlayFromStart`)
    (:`Update`
      (`SceneComponent.K2_SetRelativeLocation` (`self.StaticMesh`) (`KismetMathLibrary.MakeVector` _relativelocation_x _relativelocation_y (+ _seno _relativelocation_z)) true false))))

(fn `UserConstructionScript`
  (`parent.UserConstructionScript`))