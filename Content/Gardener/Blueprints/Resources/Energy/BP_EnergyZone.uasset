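; BP_EnergyZone is a tree-like energy zone that sends charge to an overlapping actor within a configurable sphere radius.
; A looping timer sends fixed charge messages, unpausing on overlap begin and pausing on end.
; Overlaps also toggle the emissive material colour, Niagara effect and start, loop and end sounds.
; With a nonzero duration, a rate-scaled timeline drives the mesh's Z scale, then destroys the zone.
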(event `self.ReceiveBeginPlay`
  (`|ExecutionSequence`
    (:`then_0`
      (bind _returnvalue (`KismetMaterialLibrary.CreateDynamicMaterialInstance` (`PrimitiveComponent.GetMaterial` (`self.StaticMesh`) 0)))
      (bind _output_get (set `self.treeDynamicMaterial` _returnvalue))
      (`PrimitiveComponent.SetMaterial` (`self.StaticMesh`) 0 _output_get))
    (:`then_1`
      (bind _returnvalue_2 (`KismetSystemLibrary.K2_SetTimerDelegate` (delegate `ReloadEnergyEvent`) 0.5 true))
      (set `self.timerHandler` _returnvalue_2)
      (if (not (`KismetMathLibrary.NearlyEqual_FloatFloat` (`self.areaDurationSeconds`)))
        (`TimelineComponent.SetPlayRate` (`self.zoneDurationTimeline`) (/ 1.0 (`self.areaDurationSeconds`)))
        (bind (_direction _currentduration) (`Timeline|zoneDurationTimeline` :!via `PlayFromStart`)
          (:`Update`
            (`SceneComponent.SetRelativeScale3D` (`self.StaticMesh`) (`KismetMathLibrary.MakeVector` 1.0 1.0 _currentduration)))
          (:`Finished`
            (`self.K2_DestroyActor`)))))
    (:`then_2`
      (`NiagaraComponent.SetPaused` (`self.Niagara`) true))))

(event `ReloadEnergyEvent`
  (message `/Game/Gardener/Blueprints/Interfaces/I_charging.sendCharge` (stale `self.Sphere.OnComponentBeginOverlap` OtherActor) 20.0))

(event `self.Sphere.OnComponentBeginOverlap`
  (params (OverlappedComponent :type "PrimitiveComponent Object Reference") (OtherActor :type "Actor Object Reference") (OtherComp :type "PrimitiveComponent Object Reference") (OtherBodyIndex :type Integer) (bFromSweep :type Boolean) (SweepResult :type "HitResult Structure (by ref)"))
  (`|ExecutionSequence`
    (:`then_0`
      (`MaterialInstanceDynamic.SetVectorParameterValue` (`self.treeDynamicMaterial`) "EmmisiveColor" (`KismetMathLibrary.LinearColorLerp` (struct) (struct :`R` 1.0 :`G` 0.964687 :`B` 0.078187 :`A` 1.0) 1.0))
      (`KismetSystemLibrary.K2_UnPauseTimerHandle` (`self.timerHandler`))
      (`AudioComponent.Play` (`self.EnergyTreeSource_Start`) 0.0)
      (`AudioComponent.Play` (`self.EnergyTreeSource_Loop`) 0.0))
    (:`then_1`
      (`NiagaraComponent.SetPaused` (`self.Niagara`) false))))

(event `self.Sphere.OnComponentEndOverlap`
  (params (OverlappedComponent :type "PrimitiveComponent Object Reference") (OtherActor :type "Actor Object Reference") (OtherComp :type "PrimitiveComponent Object Reference") (OtherBodyIndex :type Integer))
  (bind _niagara (`self.Niagara`))
  (`|ExecutionSequence`
    (:`then_0`
      (`MaterialInstanceDynamic.SetVectorParameterValue` (`self.treeDynamicMaterial`) "EmmisiveColor" (`KismetMathLibrary.LinearColorLerp` (struct :`R` 1.0 :`G` 0.964687 :`B` 0.078187 :`A` 1.0) (struct) 1.0))
      (`KismetSystemLibrary.K2_PauseTimerHandle` (`self.timerHandler`)))
    (:`then_1`
      (`NiagaraComponent.ResetSystem` _niagara)
      (`NiagaraComponent.SetPaused` _niagara true)
      (`AudioComponent.Play` (`self.EnergyTreeSource_End`) 0.0)
      (`AudioComponent.Stop` (`self.EnergyTreeSource_Loop`)))))

(fn `GetSendCharge`
  (params (objectReference :type "Actor Object Reference"))
  (`self.sendCharge` 0.0))

(fn `UserConstructionScript`
  (`SphereComponent.SetSphereRadius` (`self.Sphere`) (`self.area`) true))