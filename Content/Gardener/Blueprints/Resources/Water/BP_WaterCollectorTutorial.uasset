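; Tutorial water collection point that feeds resource to whatever actor stands in its Zone.
; A looping timer, created paused at BeginPlay, sends a fixed BaseResource message to the last overlapping actor.
; Zone overlap unpauses the timer, plays the collect sound loop and shows the TutorialKey prompt, while leaving reverses all three, with no actor filtering.
; Tick keeps the prompt turned toward the player camera.
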(event `self.ReceiveTick`
  (params (DeltaSeconds :type "Float (single-precision)"))
  (bind _tutorial_key (`self.Tutorial Key`))
  (`SceneComponent.K2_SetWorldRotation` _tutorial_key (`KismetMathLibrary.FindLookAtRotation` (`SceneComponent.K2_GetComponentLocation` _tutorial_key) (`SceneComponent.K2_GetComponentLocation` (`PlayerCameraManager.TransformComponent` (`GameplayStatics.GetPlayerCameraManager` 0)))) false false))

(event `self.ReceiveBeginPlay`
  (`ActorComponent.SetActive` (`self.Water_Collect_Loop`) false false)
  (`SceneComponent.SetVisibility` (`self.Tutorial Key`) false true)
  (bind _returnvalue (`KismetSystemLibrary.K2_SetTimerDelegate` (delegate `LoadResourcesEvent`) 0.5 true))
  (`KismetSystemLibrary.K2_PauseTimerHandle` _returnvalue))

(event `LoadResourcesEvent`
  (message `/Game/Gardener/Blueprints/Interfaces/I_charging.sendResource` (stale `self.Zone.OnComponentBeginOverlap` OtherActor) 10.0 (`self.baseResource`)))

(event `self.Zone.OnComponentBeginOverlap`
  (params (OverlappedComponent :type "PrimitiveComponent Object Reference") (OtherActor :type "Actor Object Reference") (OtherComp :type "PrimitiveComponent Object Reference") (OtherBodyIndex :type Integer) (bFromSweep :type Boolean) (SweepResult :type "HitResult Structure (by ref)"))
  (`AudioComponent.Play` (`self.Water_Collect_Loop`) 0.0)
  (`KismetSystemLibrary.K2_UnPauseTimerHandle` (stale `self.ReceiveBeginPlay` _returnvalue))
  (`SceneComponent.SetVisibility` (`self.Tutorial Key`) true true))

(event `self.Zone.OnComponentEndOverlap`
  (params (OverlappedComponent :type "PrimitiveComponent Object Reference") (OtherActor :type "Actor Object Reference") (OtherComp :type "PrimitiveComponent Object Reference") (OtherBodyIndex :type Integer))
  (`AudioComponent.Stop` (`self.Water_Collect_Loop`))
  (`KismetSystemLibrary.K2_PauseTimerHandle` (stale `self.ReceiveBeginPlay` _returnvalue))
  (`SceneComponent.SetVisibility` (`self.Tutorial Key`) false true))

(fn `UserConstructionScript`
  (`parent.UserConstructionScript`))