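; Base work zone for the gardener game, where water sent to it fills a job progress meter until the job completes.
; Box overlap sets or clears this zone as the work zone reference on the cached BP_Cuco player, without checking the overlapping actor.
; SendWater raises clamped progress while in use; a later call after it reaches full fires OnFilled, sound and player effect once, and tints the cube's dynamic material green.
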(event `self.ReceiveBeginPlay`
  (bind _cube (`self.Cube`))
  (bind _asbp_cuco (cast `/Game/Gardener/Blueprints/Vehicles/BP_Cuco` (`GameplayStatics.GetPlayerPawn` 0)))
  (set `self.As BP Cuco` _asbp_cuco)
  (for (_array_element _array_index) (`|MakeArray` (`PrimitiveComponent.GetMaterial` _cube 0))
    (bind _returnvalue (`PrimitiveComponent.CreateDynamicMaterialInstance` _cube _array_index _array_element "None"))
    (`KismetArrayLibrary.Array_Set` (`self.DynamicMaterial`) _array_index _returnvalue true)
    (`/Game/Gardener/Blueprints/Vehicles/BP_Cuco.WorkBaseRef` (`self.As BP Cuco`)
      (:`then`)
      (:`else`
        (`KismetSystemLibrary.PrintString` "No esta en al zona de trabajo")))))

(event `/Game/Gardener/Blueprints/Interfaces/I_charging.sendWater`
  (params (Amount :type "Float (double-precision)") (isBeingUsed :type Boolean) (resourceType :type "/Game/Gardener/Blueprints/Interfaces/Enums/EResources Enum" :default "NewEnumerator0"))
  (`KismetSystemLibrary.PrintString` "Sending Water...")
  (if isBeingUsed
    (if (`self.isCompleted`)
      (`KismetSystemLibrary.PrintString` "already")
      (`/Engine/EditorBlueprintResources/StandardMacros.DoOnce` false
        (:`Completed`
          (`|ExecutionSequence`
            (:`then_0`
              (`self.OnFilled`)
              (`GameplayStatics.PlaySound2D` "/Game/Gardener/Audio/SFX/SFX_Mision_Complete.SFX_Mision_Complete" 1.0 1.0 0.0 null null))
            (:`then_1`
              (`ActorComponent.Activate` (`/Game/Gardener/Blueprints/Vehicles/BP_Cuco.NS_WorkSpaceComplete` (`self.As BP Cuco`)) false)
              (for _array_element (`self.DynamicMaterial`)
                (`MaterialInstanceDynamic.SetVectorParameterValue` _array_element "Color" (struct :`R` 0.174858 :`G` 1.0 :`A` 1.0)))))))
      (else
        (bind _output_get (`self.growPlants` Amount))
        (set `self.isCompleted` (>= _output_get 100.0))))
    (else
      (`KismetSystemLibrary.PrintString` "isNotBeingUsed"))))

(event `self.Box.OnComponentBeginOverlap`
  (params (OverlappedComponent :type "PrimitiveComponent Object Reference") (OtherActor :type "Actor Object Reference") (OtherComp :type "PrimitiveComponent Object Reference") (OtherBodyIndex :type Integer) (bFromSweep :type Boolean) (SweepResult :type "HitResult Structure (by ref)"))
  (`KismetSystemLibrary.PrintString` "Cast to BP_BaseVehicle Succesful")
  (`|ExecutionSequence`
    (:`then_0`
      (`/Engine/EditorBlueprintResources/StandardMacros.DoOnce` false
        (:`Completed`
          (`KismetSystemLibrary.PrintString` "Los pods no se pueden usar en las zonas de trabajo jeje"))))
    (:`then_1`
      (bind _output_get (set `/Game/Gardener/Blueprints/Vehicles/BP_Cuco.WorkBaseRef` self (`self.As BP Cuco`)))
      (`KismetSystemLibrary.PrintString` (`KismetSystemLibrary.GetDisplayName` _output_get)))))

(event `self.Box.OnComponentEndOverlap`
  (params (OverlappedComponent :type "PrimitiveComponent Object Reference") (OtherActor :type "Actor Object Reference") (OtherComp :type "PrimitiveComponent Object Reference") (OtherBodyIndex :type Integer))
  (set `/Game/Gardener/Blueprints/Vehicles/BP_Cuco.WorkBaseRef` null (`self.As BP Cuco`))
  (`/Game/Gardener/Blueprints/Vehicles/BP_Cuco.WorkBaseRef` (`self.As BP Cuco`)
    (:`then`)
    (:`else`
      (`KismetSystemLibrary.PrintString` "No esta en al zona de trabajo"))))

(fn `growPlants`
  (params (amountOfResource :type "Float (double-precision)"))
  (returns (Output_Get :type "Float (double-precision)"))
  (bind _output_get (set `self.jobProgress` (`KismetMathLibrary.FClamp` (+ (`self.jobProgress`) (* amountOfResource 3.0)) 0.0 100.0)))
  (`KismetSystemLibrary.PrintString` (`KismetStringLibrary.Concat_StrStr` "Llenando: " (`KismetStringLibrary.Conv_DoubleToString` _output_get)))
  (return _output_get))

(fn `UserConstructionScript`)