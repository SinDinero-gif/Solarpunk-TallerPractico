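; BP_Garage is a level-exit trigger in the Gardener game, built on a Box overlap and gated by an IsActive flag.
; BeginPlay clears the flag and caches GM_GardnerGameMode; nothing in this Blueprint sets the flag true.
; When active, any overlap in the tutorial level calls the game mode's CallOnLevelCompleted with BabilonMap.
; Other levels only print a credits message, and end overlap does nothing.
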(event `self.ReceiveBeginPlay`
  (set `self.isActive` false)
  (bind _asgm_gardner_game_mode (cast `/Game/Gardener/Core/GM_GardnerGameMode` (`GameplayStatics.GetGameMode`)))
  (set `self.As GM Gardner Game Mode` _asgm_gardner_game_mode))

(event `self.Box.OnComponentBeginOverlap`
  (params (OverlappedComponent :type "PrimitiveComponent Object Reference") (OtherActor :type "Actor Object Reference") (OtherComp :type "PrimitiveComponent Object Reference") (OtherBodyIndex :type Integer) (bFromSweep :type Boolean) (SweepResult :type "HitResult Structure (by ref)"))
  (if (`self.isActive`)
    (`KismetSystemLibrary.PrintString` "Level Ended")
    (bind _returnvalue (`GameplayStatics.GetCurrentLevelName` true))
    (if (== _returnvalue "tutorial")
      (`/Game/Gardener/Core/GM_GardnerGameMode.OnLevelCompleted` (`self.As GM Gardner Game Mode`) "BabilonMap ")
      (else
        (`KismetSystemLibrary.PrintString` "Load Credits")))
    (else
      (`KismetSystemLibrary.PrintString` "Garage Inactive"))))

(event `self.Box.OnComponentEndOverlap`
  (params (OverlappedComponent :type "PrimitiveComponent Object Reference") (OtherActor :type "Actor Object Reference") (OtherComp :type "PrimitiveComponent Object Reference") (OtherBodyIndex :type Integer))
  (if (`self.isActive`)
    _))

(fn `UserConstructionScript`)