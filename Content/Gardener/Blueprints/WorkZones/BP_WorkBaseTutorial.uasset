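; Gardener work zone Blueprint that shows a tutorial UI component for the work base while something overlaps its box.
; Box begin and end overlap events show and hide the UI and its children, with no filter on the overlapping actor.
; Every tick, the UI rotates to face the player camera, billboard style.
; BeginPlay and construction only call the parent implementations.
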(event `self.ReceiveTick`
  (params (DeltaSeconds :type "Float (single-precision)"))
  (bind _workbaseuitutorial (`self.WorkBaseUITutorial`))
  (`SceneComponent.K2_SetWorldRotation` _workbaseuitutorial (`KismetMathLibrary.FindLookAtRotation` (`SceneComponent.K2_GetComponentLocation` _workbaseuitutorial) (`SceneComponent.K2_GetComponentLocation` (`PlayerCameraManager.TransformComponent` (`GameplayStatics.GetPlayerCameraManager` 0)))) false false))

(event `self.ReceiveBeginPlay`
  (`parent.ReceiveBeginPlay`))

(event `self.Box.OnComponentBeginOverlap`
  (params (OverlappedComponent :type "PrimitiveComponent Object Reference") (OtherActor :type "Actor Object Reference") (OtherComp :type "PrimitiveComponent Object Reference") (OtherBodyIndex :type Integer) (bFromSweep :type Boolean) (SweepResult :type "HitResult Structure (by ref)"))
  (`SceneComponent.SetVisibility` (`self.WorkBaseUITutorial`) true true))

(event `self.Box.OnComponentEndOverlap`
  (params (OverlappedComponent :type "PrimitiveComponent Object Reference") (OtherActor :type "Actor Object Reference") (OtherComp :type "PrimitiveComponent Object Reference") (OtherBodyIndex :type Integer))
  (`SceneComponent.SetVisibility` (`self.WorkBaseUITutorial`) false true))

(fn `UserConstructionScript`
  (`parent.UserConstructionScript`))